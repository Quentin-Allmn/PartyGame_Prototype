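; Press station that turns a copper, brass or zinc fusion actor into the matching ingredient actor.
; A box overlap records the fusion actor and its metal type, clearing only the actor reference on exit.
; InteractPress triggers Press, which destroys that actor and lerps the press head along a timeline.
; When the timeline finishes, the ingredient spawns at ItemLocation and is stored as Item.
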(event `Press`
  (bind (_press_down_position_x _press_down_position_y _press_down_position_z) (`KismetMathLibrary.BreakVector` (`self.Press Down Position`)))
  (bind (_press_top_position_x _press_top_position_y _press_top_position_z) (`KismetMathLibrary.BreakVector` (`self.Press Top Position`)))
  (bind _fusion__ref (`self.Fusion  Ref`))
  (`/Engine/EditorBlueprintResources/StandardMacros.IsValid` _fusion__ref
    (:`Is Valid`
      (`self.K2_DestroyActor` _fusion__ref)
      (set `self.Item` null)
      (bind (_direction _newtrack_0) (`Timeline|Timeline` :!via `PlayFromStart`)
        (:`Update`
          (`SceneComponent.K2_SetRelativeLocation` (`self.Press`) (`KismetMathLibrary.MakeVector` 0.0 0.0 (`KismetMathLibrary.Lerp` _press_top_position_z _press_down_position_z _newtrack_0)) false false))
        (:`Finished`
          (bind _new_item (`self.Spawn Actor`))
          (set `self.Item` _new_item)
          (set `self.Ingredient` "NewEnumerator3"))))))

(event `self.Box.OnComponentBeginOverlap`
  (params (OverlappedComponent :type "PrimitiveComponent Object Reference") (OtherActor :type "Actor Object Reference") (OtherComp :type "PrimitiveComponent Object Reference") (OtherBodyIndex :type Integer) (bFromSweep :type Boolean) (SweepResult :type "HitResult Structure (by ref)"))
  (bind _asbp_fusion_copper (cast `/Game/Blueprints/Ingredients/Copper/BP_Fusion_Copper` OtherActor)
    (:`then`
      (set `self.Fusion  Ref` _asbp_fusion_copper)
      (set `self.Ingredient` "NewEnumerator1"))
    (:`CastFailed`
      (bind _asbp_fusion_brass (cast `/Game/Blueprints/Ingredients/Brass/BP_Fusion_Brass` OtherActor)
        (:`then`
          (set `self.Fusion  Ref` _asbp_fusion_brass)
          (set `self.Ingredient` "NewEnumerator2"))
        (:`CastFailed`
          (bind _asbp_fusion_zinc (cast `/Game/Blueprints/Ingredients/Zinc/BP_Fusion_Zinc` OtherActor))
          (set `self.Fusion  Ref` _asbp_fusion_zinc)
          (set `self.Ingredient` "NewEnumerator0"))))))

(event `self.Box.OnComponentEndOverlap`
  (params (OverlappedComponent :type "PrimitiveComponent Object Reference") (OtherActor :type "Actor Object Reference") (OtherComp :type "PrimitiveComponent Object Reference") (OtherBodyIndex :type Integer))
  (set `self.Fusion  Ref` null))

(fn `InteractDesk`
  (returns (Desk :type "/Game/Blueprints/Tools/BP_Desk Object Reference"))
  (return null))

(fn `InteractFurnance`
  (returns (Furnance :type "/Game/Blueprints/Tools/BP_Furnance Object Reference"))
  (return null))

(fn `InteractMineralSpawner`
  (returns (`Mineral Spawner` :type "/Game/Blueprints/Tools/BP_MineralSpawner Object Reference"))
  (return null))

(fn `InteractMixer`
  (returns (Mixer :type "/Game/Blueprints/Tools/BP_Mixer Object Reference"))
  (return null))

(fn `InteractPress`
  (returns (Press :type "/Game/Blueprints/Tools/BP_Press Object Reference"))
  (`self.Press `)
  (return self))

(fn `InteractSpout`
  (returns (Spout :type "/Game/Blueprints/Tools/BP_Spout Object Reference"))
  (return null))

(fn `InteractWorkBench`
  (returns (Workbench :type "/Game/Blueprints/Tools/BP_Etabli Object Reference"))
  (return null))

(fn `Spawn Actor`
  (returns (`New Item` :type "Actor Object Reference"))
  (bind _returnvalue (`SceneComponent.K2_GetComponentToWorld` (`self.ItemLocation`)))
  (switch `/Game/Blueprints/Enums/Enum_Ingredients` (`self.Ingredient`)
    (:`NewEnumerator0`
      (bind _returnvalue_2 (`|SpawnActorFromClass` "/Game/Blueprints/Ingredients/Zinc/BP_Ingredient_Zinc.BP_Ingredient_Zinc_C" _returnvalue "Undefined" "MultiplyWithRoot" null null))
      (return _returnvalue_2))
    (:`NewEnumerator1`
      (bind _returnvalue_3 (`|SpawnActorFromClass` "/Game/Blueprints/Ingredients/Copper/BP_Ingredient_Copper.BP_Ingredient_Copper_C" _returnvalue "Undefined" "MultiplyWithRoot" null null))
      (return _returnvalue_3))
    (:`NewEnumerator2`
      (bind _returnvalue_4 (`|SpawnActorFromClass` "/Game/Blueprints/Ingredients/Brass/BP_Ingredient_Brass.BP_Ingredient_Brass_C" (`SceneComponent.K2_GetComponentToWorld` (`self.ItemLocation`)) "Undefined" "MultiplyWithRoot" null null))
      (return _returnvalue_4))))

(fn `UserConstructionScript`)