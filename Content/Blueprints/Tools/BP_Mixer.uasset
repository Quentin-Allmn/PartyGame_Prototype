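; BP_Mixer is a tool station that combines fused copper and fused zinc into brass.
; Box overlaps track the copper and zinc references and store any overlapping brass as Item.
; When both metals are present, MakeBrass destroys them and, after a short delay, spawns BP_Fusion_Brass at ItemLocation as the new Item.
; Among its per-station Interact functions, only InteractMixer returns self, identifying the actor as the mixer.
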(event `Make Brass`
  (set `self.Item` null)
  (`/Engine/EditorBlueprintResources/StandardMacros.IsValid` (`self.Ref Copper F`)
    (:`Is Valid`
      (`/Engine/EditorBlueprintResources/StandardMacros.IsValid` (`self.Ref Zinc F`)
        (:`Is Valid`
          (`self.K2_DestroyActor` (`self.Ref Zinc F`))
          (`self.K2_DestroyActor` (`self.Ref Copper F`))
          (`KismetSystemLibrary.Delay` 0.2)
          (bind _returnvalue (`|SpawnActorFromClass` "/Game/Blueprints/Ingredients/Brass/BP_Fusion_Brass.BP_Fusion_Brass_C" (`SceneComponent.K2_GetComponentToWorld` (`self.ItemLocation`)) "Undefined" "MultiplyWithRoot" null null))
          (set `self.Item` _returnvalue))))))

(event `self.Box.OnComponentBeginOverlap`
  (params (OverlappedComponent :type "PrimitiveComponent Object Reference") (OtherActor :type "Actor Object Reference") (OtherComp :type "PrimitiveComponent Object Reference") (OtherBodyIndex :type Integer) (bFromSweep :type Boolean) (SweepResult :type "HitResult Structure (by ref)"))
  (bind _asbp_fusion_copper (cast `/Game/Blueprints/Ingredients/Copper/BP_Fusion_Copper` OtherActor)
    (:`then`
      (set `self.Ref Copper F` _asbp_fusion_copper)
      (set `self.Item` null)
      (`self.Make Brass`))
    (:`CastFailed`
      (bind _asbp_fusion_zinc (cast `/Game/Blueprints/Ingredients/Zinc/BP_Fusion_Zinc` OtherActor)
        (:`then`
          (set `self.Ref Zinc F` _asbp_fusion_zinc)
          (set `self.Item` null)
          (`self.Make Brass`))
        (:`CastFailed`
          (bind _asbp_fusion_brass (cast `/Game/Blueprints/Ingredients/Brass/BP_Fusion_Brass` OtherActor))
          (set `self.Item` _asbp_fusion_brass))))))

(event `self.Box.OnComponentEndOverlap`
  (params (OverlappedComponent :type "PrimitiveComponent Object Reference") (OtherActor :type "Actor Object Reference") (OtherComp :type "PrimitiveComponent Object Reference") (OtherBodyIndex :type Integer))
  (cast `/Game/Blueprints/Ingredients/Copper/BP_Fusion_Copper` OtherActor
    (:`then`
      (set `self.Ref Copper F` null))
    (:`CastFailed`
      (cast `/Game/Blueprints/Ingredients/Zinc/BP_Fusion_Zinc` OtherActor)
      (set `self.Ref Zinc F` null))))

(fn `InteractDesk`
  (returns (Desk :type "/Game/Blueprints/Tools/BP_Desk Object Reference"))
  (return null))

(fn `InteractFurnance`
  (returns (Furnance :type "/Game/Blueprints/Tools/BP_Furnance Object Reference"))
  (return null))

(fn `InteractMixer`
  (returns (Mixer :type "/Game/Blueprints/Tools/BP_Mixer Object Reference"))
  (return self))

(fn `InteractPress`
  (returns (Press :type "/Game/Blueprints/Tools/BP_Press Object Reference"))
  (return null))

(fn `InteractSpout`
  (returns (NewParam :type "/Game/Blueprints/Tools/BP_Spout Object Reference"))
  (return null))

(fn `InteractWorkBench`
  (returns (Workbench :type "/Game/Blueprints/Tools/BP_Etabli Object Reference"))
  (return null))

(fn `UserConstructionScript`)