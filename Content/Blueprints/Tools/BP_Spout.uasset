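; BP_Spout is a crafting station that turns zinc, copper or brass fusion actors into the matching metal bar.
; A box overlap identifies the fusion type by casting and triggers Spout, which after one second destroys that actor and spawns the bar at ItemLocationR, storing it as Item.
; Other overlapping actors clear the stored ingredient and actor reference.
; Among its station interaction functions, only InteractSpout returns self.
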(event `Spout`
  (bind _ingredient (`self.Ingredient`))
  (bind _returnvalue (`SceneComponent.K2_GetComponentToWorld` (`self.ItemLocationR`)))
  (`KismetSystemLibrary.Delay` 1.0)
  (`self.K2_DestroyActor` (`self.Fusion Actor`))
  (`KismetSystemLibrary.PrintString` (`|GetEnumeratorNameAsString` _ingredient))
  (switch `/Game/Blueprints/Enum_Ingredients` _ingredient
    (:`NewEnumerator0`
      (bind _returnvalue_2 (`|SpawnActorFromClass` "/Game/Blueprints/Ingredients/Zinc/BP_Zinc_Bar.BP_Zinc_Bar_C" _returnvalue "Undefined" "MultiplyWithRoot" null null))
      (set `self.Item` _returnvalue_2))
    (:`NewEnumerator1`
      (bind _returnvalue_3 (`|SpawnActorFromClass` "/Game/Blueprints/Ingredients/Copper/BP_Copper_Bar.BP_Copper_Bar_C" _returnvalue "Undefined" "MultiplyWithRoot" null null))
      (set `self.Item` _returnvalue_3))
    (:`NewEnumerator2`
      (bind _returnvalue_4 (`|SpawnActorFromClass` "/Game/Blueprints/Ingredients/Brass/BP_Brass_Bar.BP_Brass_Bar_C" _returnvalue "Undefined" "MultiplyWithRoot" null null))
      (set `self.Item` _returnvalue_4)))
  (set `self.Ingredient` "NewEnumerator3"))

(event `self.Box.OnComponentBeginOverlap`
  (params (OverlappedComponent :type "PrimitiveComponent Object Reference") (OtherActor :type "Actor Object Reference") (OtherComp :type "PrimitiveComponent Object Reference") (OtherBodyIndex :type Integer) (bFromSweep :type Boolean) (SweepResult :type "HitResult Structure (by ref)"))
  (cast `/Game/Blueprints/Ingredients/Zinc/BP_Fusion_Zinc` OtherActor
    (:`then`
      (set `self.Ingredient` "NewEnumerator0")
      (set `self.Fusion Actor` OtherActor)
      (`self.Spout`))
    (:`CastFailed`
      (cast `/Game/Blueprints/Ingredients/Copper/BP_Fusion_Copper` OtherActor
        (:`then`
          (set `self.Ingredient` "NewEnumerator1")
          (set `self.Fusion Actor` OtherActor)
          (`self.Spout`))
        (:`CastFailed`
          (cast `/Game/Blueprints/Ingredients/Brass/BP_Fusion_Brass` OtherActor
            (:`then`
              (set `self.Ingredient` "NewEnumerator2")
              (set `self.Fusion Actor` OtherActor)
              (`self.Spout`))
            (:`CastFailed`
              (set `self.Ingredient` "NewEnumerator3")
              (set `self.Fusion Actor` null))))))))

(event `self.Box.OnComponentEndOverlap`
  (params (OverlappedComponent :type "PrimitiveComponent Object Reference") (OtherActor :type "Actor Object Reference") (OtherComp :type "PrimitiveComponent Object Reference") (OtherBodyIndex :type Integer)))

(fn `InteractDesk`
  (returns (Desk :type "/Game/Blueprints/Tools/BP_Desk Object Reference"))
  (return null))

(fn `InteractFurnance`
  (returns (Furnance :type "/Game/Blueprints/Tools/BP_Furnance Object Reference"))
  (return null))

(fn `InteractMixer`
  (returns (Mixer :type "/Game/Blueprints/Tools/BP_Mixer Object Reference"))
  (return null))

(fn `InteractPress`
  (returns (Press :type "/Game/Blueprints/Tools/BP_Press Object Reference"))
  (return null))

(fn `InteractSpout`
  (returns (Spout :type "/Game/Blueprints/Tools/BP_Spout Object Reference"))
  (return self))

(fn `InteractWorkBench`
  (returns (Workbench :type "/Game/Blueprints/Tools/BP_Etabli Object Reference"))
  (return null))

(fn `UserConstructionScript`)