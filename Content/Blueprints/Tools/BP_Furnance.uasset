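; Furnace tool that turns copper or zinc minerals into their matching fusion items.
; A mineral entering the Box overlap sets the ingredient and mineral reference, then Melt starts a short timer.
; When the timer fires, it destroys the mineral and spawns the fusion actor at ItemLocation, storing it as Item.
; Among the per-station Interact functions, only InteractFurnance returns self, identifying this actor as the furnace.
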(event `Melt`
  (`/Engine/EditorBlueprintResources/StandardMacros.IsValid` (`self.Mineral Ref`)
    (:`Is Valid`
      (set `self.Item` null)
      (`KismetSystemLibrary.K2_SetTimerDelegate` (delegate `Set Metal Fusion`) 5.0 false -1.0))))

(event `Set Metal Fusion`
  (`self.K2_DestroyActor` (`self.Mineral Ref`))
  (bind _new_item (`self.Spawn Actor`))
  (set `self.Item` _new_item)
  (set `self.Ingredient` "NewEnumerator3"))

(event `self.Box.OnComponentBeginOverlap`
  (params (OverlappedComponent :type "PrimitiveComponent Object Reference") (OtherActor :type "Actor Object Reference") (OtherComp :type "PrimitiveComponent Object Reference") (OtherBodyIndex :type Integer) (bFromSweep :type Boolean) (SweepResult :type "HitResult Structure (by ref)"))
  (bind _asbp_copper_mineral (cast `/Game/Blueprints/Ingredients/Copper/BP_Copper_Mineral` OtherActor)
    (:`then`
      (set `self.Mineral Ref` _asbp_copper_mineral)
      (set `self.Ingredient` "NewEnumerator1")
      (`self.Melt`))
    (:`CastFailed`
      (bind _asbp_zinc_mineral (cast `/Game/Blueprints/Ingredients/Zinc/BP_Zinc_Mineral` OtherActor)
        (:`then`
          (set `self.Mineral Ref` _asbp_zinc_mineral)
          (set `self.Ingredient` "NewEnumerator0")
          (`self.Melt`))
        (:`CastFailed`
          (set `self.Ingredient` "NewEnumerator3"))))))

(event `self.Box.OnComponentEndOverlap`
  (params (OverlappedComponent :type "PrimitiveComponent Object Reference") (OtherActor :type "Actor Object Reference") (OtherComp :type "PrimitiveComponent Object Reference") (OtherBodyIndex :type Integer))
  (set `self.Mineral Ref` null))

(fn `InteractDesk`
  (returns (Desk :type "/Game/Blueprints/Tools/BP_Desk Object Reference"))
  (return null))

(fn `InteractFurnance`
  (returns (Furnance :type "/Game/Blueprints/Tools/BP_Furnance Object Reference"))
  (return self))

(fn `InteractMixer`
  (returns (Mixer :type "/Game/Blueprints/Tools/BP_Mixer Object Reference"))
  (return null))

(fn `InteractPress`
  (returns (Press :type "/Game/Blueprints/Tools/BP_Press Object Reference"))
  (return null))

(fn `InteractSpout`
  (returns (Spout :type "/Game/Blueprints/Tools/BP_Spout Object Reference"))
  (return null))

(fn `InteractWorkBench`
  (returns (Workbench :type "/Game/Blueprints/Tools/BP_Etabli Object Reference"))
  (return null))

(fn `Spawn Actor`
  (returns (`New Item` :type "Actor Object Reference"))
  (bind _returnvalue (`SceneComponent.K2_GetComponentToWorld` (`self.ItemLocation`)))
  (switch `/Game/Blueprints/Enum_Ingredients` (`self.Ingredient`)
    (:`NewEnumerator0`
      (bind _returnvalue_2 (`|SpawnActorFromClass` "/Game/Blueprints/Ingredients/Zinc/BP_Fusion_Zinc.BP_Fusion_Zinc_C" _returnvalue "Undefined" "MultiplyWithRoot" null null))
      (return _returnvalue_2))
    (:`NewEnumerator1`
      (bind _returnvalue_3 (`|SpawnActorFromClass` "/Game/Blueprints/Ingredients/Copper/BP_Fusion_Copper.BP_Fusion_Copper_C" _returnvalue "Undefined" "MultiplyWithRoot" null null))
      (return _returnvalue_3))))

(fn `UserConstructionScript`)